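; Equipment component that tracks action, supply and support slots, the active slot and a holster flag, with RepNotify handlers for each.
; It stores links to container and outfit components and writes items into four clamped action slots.
; Active-slot replication broadcasts the slot's item ID when the holster flag is set.
; Holstering sets the flag owner-side and calls a server event, which is empty, as are dropping and the other notifies.
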(event `SV_Holster`
  (params (`on?` :type Boolean)))

(fn `dropFromActionSlot`
  (params (slotNumber :type Integer)))

(fn `holster`
  (params (`on?` :type Boolean))
  (bind _output_get (set `self.flagHolster` `on?`)) ; owner-side
  (`self.SV_Holster` _output_get))

(fn `LinkToContainerComponent`
  (params (Container :type "/Game/A/GameSystems/ContainerSystem/AC_Container Object Reference"))
  (`/Engine/EditorBlueprintResources/StandardMacros.IsValid` Container
    (:`Is Valid`
      (set `self.LinkedContainer` Container))))

(fn `LinkToOutfitComponent`
  (params (outfitComponent :type "/Game/A/GameSystems/OutfitSystem/CHA_Outfit Object Reference"))
  (`/Engine/EditorBlueprintResources/StandardMacros.IsValid` outfitComponent
    (:`Is Valid`
      (set `self.LinkedOutfit` outfitComponent))))

(fn `OnRep_ActionSlot`)

(fn `OnRep_currentActiveSlot`
  (if (`self.flagHolster`)
    (`self.ChangedActiveEquipment` (`.ItemID_2_DD90FB2E428E069BFFD2939AB5E103D4` (break `/Game/A/GameSystems/ContainerSystem/Item_Struct` (`|GetArrayItem` (`self.ActionSlot`) (`KismetMathLibrary.Clamp` (`self.currentActiveSlot`) 0 3)))))))

(fn `OnRep_flagHolster`)

(fn `OnRep_SupplySlot`)

(fn `OnRep_SupportSlot`)

(fn `setActionSlot`
  (params (slotNumber :type Integer) (newItemID :type Integer) (newCondition :type Integer))
  (`|VariableSetRef` (`|GetArrayItem` (`self.ActionSlot`) (`KismetMathLibrary.Clamp` slotNumber 0 3)) (make `/Game/A/GameSystems/ContainerSystem/Item_Struct` newItemID newCondition)))